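; Agent Blueprint that displays its scoring and kick statistics as in-world text.
; Every Tick, it reads scored points, kick count and false kick count through getter functions and writes each, with a label, to one of three TextRender components.
; The graphs only handle this display; BeginPlay, overlap and the construction script are empty, and the counting logic is not in this file.
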(event `self.ReceiveTick`
  (params (DeltaSeconds :type "Float (single-precision)"))
  (`TextRenderComponent.K2_SetText` (`self.TextRender`) (`KismetTextLibrary.Conv_StringToText` (`KismetStringLibrary.Concat_StrStr` "Goals: " (`KismetStringLibrary.Conv_IntToString` (`self.GetScoredPoints`)))))
  (`TextRenderComponent.K2_SetText` (`self.TextRender1`) (`KismetTextLibrary.Conv_StringToText` (`KismetStringLibrary.Concat_StrStr` "Kicks: " (`KismetStringLibrary.Conv_IntToString` (`self.GetNumberOfKicks`)))))
  (`TextRenderComponent.K2_SetText` (`self.TextRender2`) (`KismetTextLibrary.Conv_StringToText` (`KismetStringLibrary.Concat_StrStr` "False kicks: " (`KismetStringLibrary.Conv_IntToString` (`self.GetNumberOfFalseKicks`))))))

(fn `UserConstructionScript`)